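; BP_NPC is a customer NPC with Hunger and Health that leaves when its health runs out.
; Tick runs through an 8-second Delay, so hunger drops by one periodically and is printed to screen.
; Once Hunger is depleted, each step deals one damage to Health instead.
; At zero Health it prints a leaving message and destroys itself.
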(event `self.ReceiveTick`
  (params (DeltaSeconds :type "Float (single-precision)"))
  (`KismetSystemLibrary.Delay` 8.0)
  (`self.Decrease Hunger`))

(fn `Decrease Health`
  (set `self.Health` (- (`self.Health`) (`self.Damage`)))
  (if (<= (`self.Health`) 0)
    (`KismetSystemLibrary.PrintString` "Customer Leaving")
    (`self.K2_DestroyActor`)))

(fn `Decrease Hunger`
  (if (<= (`self.Hunger`) 0)
    (set `self.Damage` 1)
    (`self.Decrease Health`)
    (else
      (bind _output_get (set `self.Hunger` (- (`self.Hunger`) 1)))
      (`KismetSystemLibrary.PrintString` (`KismetTextLibrary.Conv_TextToString` (`|FormatText` "Hunger-{Hunger}" (`KismetTextLibrary.Conv_IntToText` _output_get)))))))

(fn `UserConstructionScript`)